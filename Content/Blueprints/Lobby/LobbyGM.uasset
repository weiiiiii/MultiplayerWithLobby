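; LobbyGM is the lobby game mode Blueprint, which currently only logs player connection events on screen.
; PostLogin prints the display name of each joining player controller.
; OnSwapPlayerControllers casts both controllers' PlayerStates to AllPlayerState and prints the old and new OwningPlayerName, with red error messages when either cast fails.
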(event `self.K2_PostLogin`
  (params (NewPlayer :type "PlayerController Object Reference"))
  (`KismetSystemLibrary.PrintString` (`KismetSystemLibrary.GetDisplayName` NewPlayer)))

(event `self.K2_OnSwapPlayerControllers`
  (params (OldPC :type "PlayerController Object Reference") (NewPC :type "PlayerController Object Reference"))
  (bind _asall_player_state (cast `/Game/Blueprints/AllLevels/AllPlayerState` (`Controller.PlayerState` OldPC))
    (:`then`
      (bind _asall_player_state_2 (cast `/Game/Blueprints/AllLevels/AllPlayerState` (`Controller.PlayerState` NewPC))
        (:`then`
          (`KismetSystemLibrary.PrintString` (`KismetStringLibrary.Concat_StrStr` "LobbyGM : Swap Controller : Old Name [" (`/Game/Blueprints/AllLevels/AllPlayerState.Owning_Player_Name` _asall_player_state) "] New Name [" (`/Game/Blueprints/AllLevels/AllPlayerState.Owning_Player_Name` _asall_player_state_2) "]") true true (struct :`R` 1.0 :`G` 0.393402 :`A` 1.0) 20.0))
        (:`CastFailed`
          (`KismetSystemLibrary.PrintString` "New PC's player state cast failed!" true true (struct :`R` 1.0 :`A` 1.0) 20.0))))
    (:`CastFailed`
      (`KismetSystemLibrary.PrintString` "Old PC's player state cast failed!" true true (struct :`R` 1.0 :`A` 1.0) 20.0))))

(fn `UserConstructionScript`)